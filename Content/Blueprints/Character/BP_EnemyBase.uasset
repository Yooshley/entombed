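; Base enemy Blueprint that handles loot drops and a material dissolve effect.
; SpawnLoot pulls items from the loot tiers, spreads rotations evenly around the enemy, then spawns one item per looping timer tick at a random distance.
; Spawned EntombedEffectActors receive the enemy's level, and a timeline drives the Dissolve parameter on supplied dynamic materials.
; UpdateFacingTarget is empty; its motion-warping update is disconnected.
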(event `self.SpawnLoot`
  (bind _returnvalue (`EntombedAbilitySystemLibrary.GetLootTiers` null))
  (`/Engine/EditorBlueprintResources/StandardMacros.IsValid` _returnvalue
    (:`Is Valid`
      (bind _returnvalue_2 (`LootTiers.GetLootItems` _returnvalue))
      (bind _output_get (set `self.LootItems` _returnvalue_2))
      (set `self.LootRotations` (`self.GetLootRotations` _output_get))
      (set `self.SpawnLootCount` 0)
      (bind _returnvalue_3 (`KismetSystemLibrary.K2_SetTimerDelegate` (delegate `SpawnLootItem`) 0.1 true))
      (set `self.LootTimerHandler` _returnvalue_3)
      (`self.SpawnLootItem`))))

(event `SpawnLootItem`
  (bind (_lootclass _blootleveloverride) (break `LootItem` (`|GetArrayItem` (`self.LootItems`) (`self.SpawnLootCount`))))
  (if (< (`self.SpawnLootCount`) (`KismetArrayLibrary.Array_Length` (`self.LootItems`)))
    (bind _returnvalue (`|SpawnActorFromClass` _lootclass (`self.GetLootTransform` (`self.SpawnLootCount`)) "AlwaysSpawn" "MultiplyWithRoot" null null))
    (if _blootleveloverride
      _
      (else
        _))
    (`/Engine/EditorBlueprintResources/StandardMacros.IncrementInt` (`self.SpawnLootCount`)
      (:`  `
        (bind _asentombed_effect_actor (cast `EntombedEffectActor` _returnvalue))
        (`/Engine/EditorBlueprintResources/StandardMacros.IsValid` _asentombed_effect_actor
          (:`Is Valid`
            (set `EntombedEffectActor.ActorLevel` (`KismetMathLibrary.Conv_IntToDouble` (`self.Level`)) _asentombed_effect_actor)))))
    (else
      (`KismetSystemLibrary.K2_ClearAndInvalidateTimerHandle` (`self.LootTimerHandler`)))))

(event `self.StartDissolveTimeline`
  (params (DynamicMaterialInstances :type "Array of MaterialInstanceDynamic Object Reference (by ref)"))
  (bind (_direction _dissolvetrack) (`Timeline|DissolveTimeline`)
    (:`Update`
      (for _array_element DynamicMaterialInstances
        (`MaterialInstanceDynamic.SetScalarParameterValue` _array_element "Dissolve" _dissolvetrack)))))

(event `self.UpdateFacingTarget`
  (params (Target :type "Vector Structure (by ref)")))

(fn `GetLootRotations`
  (params (TargetArray :type "Array of LootItem Structure (by ref)"))
  (returns (ReturnValue :type "Array of Rotator Structure"))
  (return (`EntombedAbilitySystemLibrary.GetEvenlySpreadRotators` (`self.GetActorForwardVector`) (`KismetMathLibrary.Vector_Up`) 360.0 (`KismetArrayLibrary.Array_Length` TargetArray))))

(fn `GetLootTransform`
  (params (LootCount :type Integer))
  (returns (LootTransform :type "Transform Structure"))
  (bind _output (`|GetArrayItem` (`self.LootRotations`) LootCount))
  (return (`KismetMathLibrary.MakeTransform` (+ (`self.K2_GetActorLocation`) (* (`KismetMathLibrary.RandomFloatInRange` (`self.MinSpawnDistance`) (`self.MaxSpawnDistance`)) (`KismetMathLibrary.GetForwardVector` _output))) _output)))

(fn `UserConstructionScript`)