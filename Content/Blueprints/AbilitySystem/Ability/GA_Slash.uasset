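; GA_Slash is a gameplay ability that plays a main-hand slice montage and spawns a projectile when the montage's slice event arrives.
; Player avatars aim through cursor target data, while other avatars use their target actor's location, and both paths share the montage logic.
; The montage blending out or being cut short ends the ability, and OnEndAbility switches the avatar's orientation mode off.
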(event `self.K2_ActivateAbility`
  (`self.K2_CommitAbility`)
  (if (`KismetSystemLibrary.DoesImplementInterface` (`self.GetAvatarActorFromActorInfo`) "/Script/entombed.PlayerInterface")
    (bind (_asynctaskproxy _datahandle) (`TargetDataUnderCursor.CreateTargetDataUnderCursor`)
      (:`ValidData`
        (`self.SetTarget` (`.Location` (`GameplayStatics.BreakHitResult` (`AbilitySystemBlueprintLibrary.GetHitResultFromTargetData` _datahandle))))))
    (else
      (bind _returnvalue (message `CombatInterface.GetTarget` (`self.GetAvatarActorFromActorInfo`)))
      (`/Engine/EditorBlueprintResources/StandardMacros.IsValid` _returnvalue
        (:`Is Valid`
          (`self.SetTarget` (`Actor.K2_GetActorLocation` _returnvalue))))))
  (`AbilityTask_PlayMontageAndWait.CreatePlayMontageAndWaitProxy` "None" "/Game/Assets/Characters/CharacterBase/Mannequin_Medium/Animations/Rig_Medium_CombatMelee/AM_Mainhand_Slice.AM_Mainhand_Slice" 1.0 "None" false
    (:`then`
      (`AbilityTask_WaitGameplayEvent.WaitGameplayEvent` (struct :`TagName` "Montage.MainHand.Slice") null
        (:`EventReceived`
          (`self.SpawnProjectile` (`self.Socket Tag`)))))
    (:`OnBlendOut`
      (`self.K2_EndAbility` :!label _label))
    (:`OnInterrupted`
      (goto _label))
    (:`OnCancelled`
      (goto _label))))

(event `self.K2_OnEndAbility`
  (params (bWasCancelled :type Boolean))
  (message `CombatInterface.SetOrientationMode` (`self.GetAvatarActorFromActorInfo`) false))