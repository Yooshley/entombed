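; GA_Swipe is a gameplay ability that plays a main-hand slice montage and launches a projectile toward the location under the cursor.
; After committing, it takes cursor target data, sets the target and starts the montage.
; A gameplay event wait times the projectile spawn at a socket to the slice event.
; Montage blend-out, interruption or cancellation ends the ability, and ending it switches off the avatar's orientation mode.
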(event `self.K2_ActivateAbility`
  (`self.K2_CommitAbility`)
  (bind (_asynctaskproxy _datahandle) (`TargetDataUnderCursor.CreateTargetDataUnderCursor`)
    (:`ValidData`
      (`self.SetTarget` (`.Location` (`GameplayStatics.BreakHitResult` (`AbilitySystemBlueprintLibrary.GetHitResultFromTargetData` _datahandle))))
      (`AbilityTask_PlayMontageAndWait.CreatePlayMontageAndWaitProxy` "None" "/Game/Assets/Characters/CharacterBase/Mannequin_Medium/Animations/Rig_Medium_CombatMelee/AM_Mainhand_Slice.AM_Mainhand_Slice" 1.0 "None" false
        (:`then`
          (`AbilityTask_WaitGameplayEvent.WaitGameplayEvent` (struct :`TagName` "Montage.MainHand.Slice") null
            (:`EventReceived`
              (`self.SpawnProjectile` (`self.Socket Tag`)))))
        (:`OnBlendOut`
          (`self.K2_EndAbility` :!label _label))
        (:`OnInterrupted`
          (goto _label))
        (:`OnCancelled`
          (goto _label))))))

(event `self.K2_OnEndAbility`
  (params (bWasCancelled :type Boolean))
  (message `CombatInterface.SetOrientationMode` (`self.GetAvatarActorFromActorInfo`) false))