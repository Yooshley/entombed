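; Gameplay ability for enemy ranged attacks that fires a projectile at the target provided by the avatar.
; It caches the target's location, then plays a random tagged montage from the avatar's CombatInterface.
; A montage-tag gameplay event spawns the projectile at a socket tag; blend-out, interruption or cancellation ends the ability.
; Montage, event tag and socket tag each come from separate Random lookups, so they can mismatch when several montages exist.
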(event `self.K2_ActivateAbility`
  (bind _returnvalue (`self.GetAvatarActorFromActorInfo`))
  (bind _returnvalue_2 (message `CombatInterface.GetTarget` _returnvalue))
  (bind _ascombat_interface (cast `CombatInterface` _returnvalue))
  (`self.SetProjectileTarget` (`Actor.K2_GetActorLocation` _returnvalue_2))
  (bind _returnvalue_3 (`CombatInterface.GetTaggedMontages` _ascombat_interface))
  (bind (_montage _sockettag _montagetag) (break `TaggedMontage` (`KismetArrayLibrary.Array_Random` _returnvalue_3)))
  (`AbilityTask_PlayMontageAndWait.CreatePlayMontageAndWaitProxy` "None" _montage
    (:`then`
      (`AbilityTask_WaitGameplayEvent.WaitGameplayEvent` _montagetag null true
        (:`EventReceived`
          (`self.SpawnProjectile` _sockettag))))
    (:`OnBlendOut`
      (`self.K2_EndAbility` :!label _label))
    (:`OnInterrupted`
      (goto _label))
    (:`OnCancelled`
      (goto _label))))