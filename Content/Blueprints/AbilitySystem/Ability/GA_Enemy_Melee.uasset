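; Gameplay ability for enemy melee attacks, played as a random tagged montage from the avatar's combat interface.
; It turns the avatar toward its target, then waits for the montage's gameplay event tag.
; On that event it damages non-ally live players within a small radius of the tagged socket and fires an impact cue at the target on a hit.
; The ability ends when the montage blends out, is interrupted or is cancelled.
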(event `self.K2_ActivateAbility`
  (bind _returnvalue (`self.GetAvatarActorFromActorInfo`))
  (bind _targetactor (`self.TargetActor`))
  (bind _returnvalue_2 (message `CombatInterface.GetTarget` (`self.GetAvatarActorFromActorInfo`)))
  (set `self.TargetActor` _returnvalue_2)
  (bind _ascombat_interface (cast `CombatInterface` (`self.GetAvatarActorFromActorInfo`)))
  (set `self.SourceCombatInterface` _ascombat_interface)
  (message `CombatInterface.SetTargetDirection` (`self.GetAvatarActorFromActorInfo`) (`Actor.K2_GetActorLocation` (`self.TargetActor`)))
  (bind _returnvalue_3 (`CombatInterface.GetTaggedMontages` (`self.SourceCombatInterface`)))
  (bind _output_get (set `self.TaggedMontage` (`KismetArrayLibrary.Array_Random` _returnvalue_3)))
  (bind (_montage _sockettag _montagetag) (break `TaggedMontage` _output_get))
  (`AbilityTask_PlayMontageAndWait.CreatePlayMontageAndWaitProxy` "None" _montage
    (:`then`
      (`AbilityTask_WaitGameplayEvent.WaitGameplayEvent` _montagetag null
        (:`EventReceived`
          (bind _returnvalue_4 (message `CombatInterface.GetCombatSocketLocation` _returnvalue _sockettag))
          (set `self.HasHitTarget` false)
          (bind _outoverlappingactors (`EntombedAbilitySystemLibrary.GetLivePlayersWithinRadius` self (`|MakeArray` _returnvalue) 50.0 _returnvalue_4))
          (for _array_element _outoverlappingactors
            (if (not (`EntombedAbilitySystemLibrary.IsAlly` (`self.GetAvatarActorFromActorInfo`) _array_element))
              (`self.CauseDamage` _array_element)
              (set `self.HasHitTarget` true)))
          (if (`self.HasHitTarget`)
            (`self.K2_ExecuteGameplayCueWithParams` (struct :`TagName` "GameplayCue.Impact") (`AbilitySystemBlueprintLibrary.MakeGameplayCueParameters` 0.0 0.0 (struct) (struct) (struct) (`BlueprintGameplayTagLibrary.MakeGameplayTagContainerFromTag` (`.MontageTag` (break `TaggedMontage` (`self.TaggedMontage`)))) (struct) (`Actor.K2_GetActorLocation` _targetactor) (0.0 0.0 0.0) null (`self.GetAvatarActorFromActorInfo`) _targetactor))))))
    (:`OnBlendOut`
      (`self.K2_EndAbility` :!label _label))
    (:`OnInterrupted`
      (goto _label))
    (:`OnCancelled`
      (goto _label))))