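; Arcane Shards gameplay ability: shows a magic circle, waits for a press, then strikes ground points around the cursor location.
; A spawned BP_PointCollection supplies one randomly rotated point per ability level while the cast montage plays.
; On the montage's cast event, cooldown commits and a looping timer steps through the points.
; Each shard applies radial damage to nearby live actors, fires a GameplayCue and commits cost.
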(event `self.K2_ActivateAbility`
  (`|ExecutionSequence`
    (:`then_0`
      (message `PlayerInterface.ShowMagicCircle` (`self.GetAvatarActorFromActorInfo`) null))
    (:`then_1`
      (`AbilityTask_WaitInputPress.WaitInputPress` false
        (:`OnPress`
          (bind (_asynctaskproxy _datahandle) (`TargetDataUnderCursor.CreateTargetDataUnderCursor`)
            (:`ValidData`
              (bind _output_get (set `self.CursorLocation` (`.ImpactPoint` (`GameplayStatics.BreakHitResult` (`AbilitySystemBlueprintLibrary.GetHitResultFromTargetData` _datahandle)))))
              (bind _returnvalue (`|SpawnActorFromClass` "/Game/Blueprints/AbilitySystem/Ability/Arcane/BP_PointCollection.BP_PointCollection_C" (`KismetMathLibrary.MakeTransform` _output_get) "AlwaysSpawn" "MultiplyWithRoot" null null))
              (bind _output_get_2 (set `self.NumPoints` (`self.GetAbilityLevel`)))
              (bind _output_get_3 (set `self.PointCollection` _returnvalue))
              (set `self.GroundPoints` (`PointCollection.GetGroundPoints` _output_get_3 (`self.CursorLocation`) _output_get_2 (`KismetMathLibrary.RandomFloatInRange` 0.0 360.0)))
              (message `CombatInterface.SetTargetDirection` (`self.GetAvatarActorFromActorInfo`) (`self.CursorLocation`))
              (`AbilityTask_PlayMontageAndWait.CreatePlayMontageAndWaitProxy` "None" "/Game/Assets/Characters/CharacterBase/Mannequin_Medium/Animations/Rig_Medium_CombatRanged/AM_MainHand_Cast.AM_MainHand_Cast" 1.0 "None" false
                (:`then`
                  (`AbilityTask_WaitGameplayEvent.WaitGameplayEvent` (struct :`TagName` "Montage.MainHand.Cast") null
                    (:`EventReceived`
                      (bind _returnvalue_2 (`KismetSystemLibrary.K2_SetTimerDelegate` (delegate `SpawnShard`) (`self.ShardSpawnDeltaTime`) true true))
                      (set `self.ShardSpawnTimer` _returnvalue_2)
                      (`self.SpawnShard`)
                      (message `PlayerInterface.HideMagicCircle` (`self.GetAvatarActorFromActorInfo`))
                      (`self.K2_CommitAbilityCooldown` false))))))))))))

(event `SpawnShard`
  (bind _returnvalue (`self.GetAvatarActorFromActorInfo`))
  (if (< (`self.Count`) (`self.NumPoints`))
    (bind _output_get (set `self.ShardSpawnLocation` (`SceneComponent.K2_GetComponentLocation` (`|GetArrayItem` (`self.GroundPoints`) (`self.Count`)))))
    (bind _outoverlappingactors (`EntombedAbilitySystemLibrary.GetLiveActorsWithinRadius` _returnvalue (`|MakeArray` _returnvalue) (`self.RadialDamageOuterRadius`) _output_get))
    (bind _output_get_2 (set `self.Out Overlapping Actors` _outoverlappingactors))
    (for _array_element _output_get_2
      (bind _structout (setmembers `DamageEffectParameters` :`StructRef` (`self.MakeDamageParametersFromClassDefaults` _array_element) :`RadialDamageOrigin` (`self.ShardSpawnLocation`)))
      (`EntombedAbilitySystemLibrary.ApplyDamageEffect` _structout))
    (`/Engine/EditorBlueprintResources/StandardMacros.IncrementInt` (`self.Count`)
      (:`  `
        (`GameplayCueFunctionLibrary.ExecuteGameplayCueOnActor` (`self.GetAvatarActorFromActorInfo`) (struct :`TagName` "GameplayCue.ArcaneShards") (`AbilitySystemBlueprintLibrary.MakeGameplayCueParameters` 0.0 0.0 (struct) (struct) (struct) (struct) (struct) (`self.ShardSpawnLocation`)))
        (`self.K2_CommitAbilityCost` false)))
    (else
      (`KismetSystemLibrary.K2_ClearAndInvalidateTimerHandle` (`self.ShardSpawnTimer`))
      (`KismetSystemLibrary.Delay` 0.2)
      (`Actor.K2_DestroyActor` (`self.PointCollection`))
      (`self.K2_EndAbility`))))