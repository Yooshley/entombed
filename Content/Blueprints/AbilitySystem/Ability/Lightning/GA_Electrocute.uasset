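; Channeled lightning ability that shocks the target under the cursor and chains beams to additional targets.
; After the channeling montage, it locks movement and adds looping ShockLoop cues, linking secondary targets to the primary.
; A looping timer commits cost and damages all stored targets, ending when cost fails.
; Input release ends it after a minimum hold, restoring movement, committing cooldown, clearing cues and applying a final damage effect to the primary.
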(event `self.K2_ActivateAbility`
  (if (`KismetSystemLibrary.DoesImplementInterface` (`self.GetAvatarActorFromActorInfo`) "/Script/entombed.CombatInterface")
    (bind (_asynctaskproxy _datahandle) (`TargetDataUnderCursor.CreateTargetDataUnderCursor`)
      (:`ValidData`
        (`self.StoreCursorDataInfo` (`AbilitySystemBlueprintLibrary.GetHitResultFromTargetData` _datahandle))
        (`self.StoreOwnerVariables`)
        (`|ExecutionSequence`
          (:`then_0`
            (set `PlayerController.bShowMouseCursor` false (`self.OwnerPlayerController`))
            (message `CombatInterface.SetTargetDirection` (`self.GetAvatarActorFromActorInfo`) (`self.CursorHitLocation`))
            (`self.K2_ExecuteGameplayCue` (struct :`TagName` "GameplayCue.ShockBurst"))
            (`AbilityTask_PlayMontageAndWait.CreatePlayMontageAndWaitProxy` "None" "/Game/Assets/Characters/CharacterBase/Mannequin_Medium/Animations/Rig_Medium_CombatRanged/AM_Channeling.AM_Channeling"
              (:`OnCompleted`
                _)
              (:`OnBlendOut`
                _)
              (:`OnInterrupted`
                _)
              (:`OnCancelled`
                _))
            (message `CombatInterface.SetCasting` (`self.GetAvatarActorFromActorInfo`) true)
            (`CharacterMovementComponent.DisableMovement` (`Character.CharacterMovement` (`self.OwnerCharacter`)))
            (`self.SpawnBeam`)
            (bind _returnvalue (`KismetSystemLibrary.K2_SetTimerDelegate` (delegate `Damage`) (`self.DamageDeltaTime`) true))
            (set `self.DamageTimerHandle` _returnvalue))
          (:`then_1`
            (bind (_asynctaskproxy_2 _timeheld) (`AbilityTask_WaitInputRelease.WaitInputRelease` false)
              (:`OnRelease`
                (bind _output_get (set `self.Time Held` _timeheld))
                (if (< _output_get (`self.MinAbilityTime`))
                  (`KismetSystemLibrary.Delay` (- (`self.MinAbilityTime`) (`self.Time Held`))))
                (`self.K2_EndAbility`)))))))
    (else
      (`self.K2_EndAbility`))))

(event `Damage`
  (bind _returnvalue (`self.K2_CommitAbilityCost` false))
  (if _returnvalue
    (if (not (`self.TargetDead`))
      (`self.ApplyDamageToAllTargets`))
    (else
      (`self.K2_EndAbility`))))

(event `self.K2_OnEndAbility`
  (params (bWasCancelled :type Boolean))
  (set `PlayerController.bShowMouseCursor` true (`self.OwnerPlayerController`))
  (message `CombatInterface.SetCasting` (`self.GetAvatarActorFromActorInfo`) false)
  (`CharacterMovementComponent.SetMovementMode` (`Character.CharacterMovement` (`self.OwnerCharacter`)) "MOVE_Walking" 0)
  (`KismetSystemLibrary.K2_ClearAndInvalidateTimerHandle` (`self.DamageTimerHandle`))
  (`self.K2_CommitAbilityCooldown` false)
  (`self.RemoveCues`)
  (`BlueprintMapLibrary.Map_Clear` (`self.AdditionalActorToCueParams`))
  (set `self.CursorHitActor` null)
  (set `self.FirstTargetImplementsInterface` false)
  (set `self.Time Held` 0.0))

(event `self.PrimaryTargetDead`
  (params (DeadActor :type "Actor Object Reference"))
  (`GameplayCueFunctionLibrary.RemoveGameplayCueOnActor` DeadActor (struct :`TagName` "GameplayCue.ShockLoop") (`self.FirstTargetCueParams`)))

(event `self.AdditionalTargetDead`
  (params (DeadActor :type "Actor Object Reference"))
  (bind (_value _returnvalue) (`BlueprintMapLibrary.Map_Find` (`self.AdditionalActorToCueParams`) DeadActor))
  (if _returnvalue
    (`GameplayCueFunctionLibrary.RemoveGameplayCueOnActor` DeadActor (struct :`TagName` "GameplayCue.ShockLoop") _value)
    (`BlueprintMapLibrary.Map_Remove` (`self.AdditionalActorToCueParams`) DeadActor)))

(fn `AddLoopCueToAdditionalTarget`
  (params (AdditionalActor :type "Actor Object Reference"))
  (bind _additionalactor (`local.AdditionalActor`))
  (bind _returnvalue (`AbilitySystemBlueprintLibrary.MakeGameplayCueParameters` 0.0 0.0 (struct) (struct) (struct) (struct) (struct) (`Actor.K2_GetActorLocation` _additionalactor) (0.0 0.0 0.0) null null _additionalactor null 1 1 (`Actor.RootComponent` (`self.CursorHitActor`))))
  (`BlueprintMapLibrary.Map_Add` (`self.AdditionalActorToCueParams`) AdditionalActor _returnvalue)
  (`GameplayCueFunctionLibrary.AddGameplayCueOnActor` (`local.AdditionalActor`) (struct :`TagName` "GameplayCue.ShockLoop") _returnvalue))

(fn `ApplyDamageToAllTargets`
  (`self.ApplyDamageToTarget` (`self.CursorHitActor`))
  (bind _keypin (`|MapForEach` (`self.AdditionalActorToCueParams`))
    (:`then`
      (`self.ApplyDamageToTarget` _keypin))))

(fn `ApplyDamageToTarget`
  (params (Actor :type "Actor Object Reference"))
  (locals (ASC :type "AbilitySystemComponent Object Reference"))
  (bind _returnvalue (`AbilitySystemBlueprintLibrary.GetAbilitySystemComponent` (`local.Actor`)))
  (`/Engine/EditorBlueprintResources/StandardMacros.IsValid` Actor
    (:`Is Valid`
      (bind _output_get (set `local.ASC` (`self.GetAbilitySystemComponentFromActorInfo`)))
      (`/Engine/EditorBlueprintResources/StandardMacros.IsValid` _output_get
        (:`Is Valid`
          (bind _returnvalue_2 (`AbilitySystemBlueprintLibrary.AssignTagSetByCallerMagnitude` (`AbilitySystemComponent.MakeOutgoingSpec` (`local.ASC`) (`self.DamageEffectClass`) (`KismetMathLibrary.Conv_IntToDouble` (`self.GetAbilityLevel`)) (`AbilitySystemComponent.MakeEffectContext` _output_get)) (struct :`TagName` "Damage.Shock")))
          (`/Engine/EditorBlueprintResources/StandardMacros.IsValid` _returnvalue
            (:`Is Valid`
              (`AbilitySystemComponent.BP_ApplyGameplayEffectSpecToSelf` _returnvalue _returnvalue_2))))))))

(fn `RemoveCues`
  (bind _cursorhitactor (`self.CursorHitActor`))
  (if (`self.FirstTargetImplementsInterface`)
    (`GameplayCueFunctionLibrary.RemoveGameplayCueOnActor` _cursorhitactor (struct :`TagName` "GameplayCue.ShockLoop") (`self.FirstTargetCueParams`))
    (`EntombedAbilitySystemLibrary.ApplyDamageEffect` (`self.MakeDamageParametersFromClassDefaults` _cursorhitactor))
    (bind (_keypin _valuepin) (`|MapForEach` (`self.AdditionalActorToCueParams`))
      (:`then`
        (`GameplayCueFunctionLibrary.RemoveGameplayCueOnActor` _keypin (struct :`TagName` "GameplayCue.ShockLoop") _valuepin)))
    (else
      (`GameplayCueFunctionLibrary.RemoveGameplayCueOnActor` (`self.GetAvatarActorFromActorInfo`) (struct :`TagName` "GameplayCue.ShockLoop") (`self.FirstTargetCueParams`)))))

(fn `SpawnBeam`
  (locals (CueTarget :type "Actor Object Reference"))
  (`self.TraceFirstTarget` (`self.CursorHitLocation`))
  (bind _returnvalue (message `CombatInterface.GetMainHandEquipment` (`self.OwnerCharacter`)))
  (set `self.FirstTargetCueParams` (`AbilitySystemBlueprintLibrary.MakeGameplayCueParameters` 0.0 0.0 (struct) (struct) (struct) (struct) (struct) (`self.CursorHitLocation`) (0.0 0.0 0.0) null null (`self.CursorHitActor`) null 1 1 _returnvalue))
  (bind _output_get (set `self.FirstTargetImplementsInterface` (`KismetSystemLibrary.DoesImplementInterface` (`self.CursorHitActor`) "/Script/entombed.CombatInterface")))
  (if _output_get
    (set `local.CueTarget` (`self.CursorHitActor`))
    (else
      (set `local.CueTarget` (`self.GetAvatarActorFromActorInfo`))))
  (`GameplayCueFunctionLibrary.AddGameplayCueOnActor` (`local.CueTarget`) (struct :`TagName` "GameplayCue.ShockLoop") (`self.FirstTargetCueParams`))
  (if (`self.FirstTargetImplementsInterface`)
    (bind _outadditionaltargets (`self.StoreAdditionalTargets`))
    (for _array_element _outadditionaltargets
      (`self.AddLoopCueToAdditionalTarget` _array_element))))