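; BP_FireBolt is the fire bolt actor of the Fire ability set, which explodes once it stops moving.
; Each Tick it measures the distance moved since the previous frame instead of handling hit or overlap events in the graph.
; When that distance is at or below MinDistancePerFrame, it plays the impact sound, spawns the NS_FireExplosion effect at its location and destroys itself.
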(event `self.ReceiveTick`
  (params (DeltaSeconds :type "Float (single-precision)"))
  (bind _locationthisframe (`self.LocationThisFrame`))
  (set `self.LocationLastFrame` (`self.LocationThisFrame`))
  (bind _output_get (set `self.LocationThisFrame` (`self.K2_GetActorLocation`)))
  (if (<= (`KismetMathLibrary.VSize` (- _output_get (`self.LocationLastFrame`))) (`self.MinDistancePerFrame`))
    (`GameplayStatics.SpawnSoundAtLocation` "/Game/Assets/Audio/Sounds/Abilities/FireBolt/sfx_FireBolt_Impact.sfx_FireBolt_Impact" _locationthisframe (struct) 1.0 1.0 0.0 null null)
    (`NiagaraFunctionLibrary.SpawnSystemAtLocation` "/Game/Assets/Effects/Projectiles/FireExplosion/NS_FireExplosion.NS_FireExplosion" _locationthisframe)
    (`self.K2_DestroyActor`)))

(fn `UserConstructionScript`)