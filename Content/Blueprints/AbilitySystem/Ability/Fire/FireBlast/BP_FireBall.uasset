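; Fireball actor for the FireBlast ability that flies outward, boomerangs back to its instigator and explodes on nearing them.
; On authority, two chained timelines lerp its location forward along its facing, then back toward the instigator's live position.
; Within the explode distance it calls OnHit, applies radial damage with outward knockback and death impulse to nearby live actors, excluding its owner, then destroys itself.
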(event `self.StartOutgoingTimeline`
  (bind _array (`|MakeArray` (`self.GetOwner`)))
  (`/Engine/EditorBlueprintResources/ActorMacros.Switch Has Authority`
    (:`Authority`
      (bind _output_get (set `self.InitialLocation` (`self.K2_GetActorLocation`)))
      (set `self.FarthestLocation` (+ _output_get (* (`self.GetActorForwardVector`) (`self.TravelDistance`))))
      (bind (_direction _outgoingtrack) (`Timeline|OutgoingTimeline`)
        (:`Update`
          (`self.K2_SetActorLocation` (`KismetMathLibrary.VLerp` (`self.InitialLocation`) (`self.FarthestLocation`) _outgoingtrack)))
        (:`Finished`
          (bind (_direction_2 _returningtrack) (`Timeline|ReturningTimeline`)
            (:`Update`
              (`self.K2_SetActorLocation` (`KismetMathLibrary.VLerp` (`self.FarthestLocation`) (`self.K2_GetActorLocation` (`self.GetInstigator`)) _returningtrack))
              (if (`self.ShouldExplode`)
                (`self.OnHit`)
                (`KismetArrayLibrary.Array_Add` _array self)
                (bind _outoverlappingactors (`EntombedAbilitySystemLibrary.GetLiveActorsWithinRadius` self _array 250.0 (`self.K2_GetActorLocation`)))
                (setmembers `DamageEffectParameters` :`StructRef` (`self.ExplosionDamageParams`) :`bIsRadialDamage` true :`RadialDamageInnerRadius` 0.0 :`RadialDamageOuterRadius` 0.0 :`RadialDamageOrigin` (`self.K2_GetActorLocation`))
                (for _array_element _outoverlappingactors
                  (bind _returnvalue (- (`self.K2_GetActorLocation` _array_element) (`self.K2_GetActorLocation`)))
                  (bind _structout (setmembers `DamageEffectParameters` :`StructRef` (`self.ExplosionDamageParams`) :`TargetAbilitySystemComponent` (`AbilitySystemBlueprintLibrary.GetAbilitySystemComponent` _array_element) :`DeathImpulseMagnitude` 500.0 :`DeathImpulse` _returnvalue :`KnockbackMagnitude` 1000.0 :`KnockbackVector` _returnvalue))
                  (`EntombedAbilitySystemLibrary.ApplyDamageEffect` _structout))
                (`self.K2_DestroyActor`)))))))))

(fn `ShouldExplode`
  (returns (ReturnValue :type Boolean))
  (return (<= (`KismetMathLibrary.VSize` (- (`self.K2_GetActorLocation`) (`self.K2_GetActorLocation` (`self.GetInstigator`)))) (`self.ExplodeDistance`))))

(fn `UserConstructionScript`)