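; Base pickup actor for potions that animates its spawn drop and plays sounds on spawn, during the drop and on destruction.
; A timeline scales the actor and offsets its height from the initial location by DropApex, playing PickupSound once when the drop curve dips below zero.
; When the timeline finishes it starts sinusoidal movement and rotation, while Tick applies the calculated location and rotation.
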(event `self.ReceiveBeginPlay`
  (`GameplayStatics.PlaySoundAtLocation` (`self.SpawnSound`) (`self.K2_GetActorLocation`) (struct) 1.0 1.0 0.0 null null null null)
  (bind (_direction _drop _scale) (`Timeline|PickupDropTimeline`)
    (:`Update`
      (set `self.CalculatedLocation` (`self.CalculateDrop` _drop))
      (`self.SetActorScale3D` (`KismetMathLibrary.MakeVector` _scale _scale _scale))
      (if (< _drop 0.0)
        (`/Engine/EditorBlueprintResources/StandardMacros.DoOnce` false
          (:`Completed`
            (`GameplayStatics.PlaySoundAtLocation` (`self.PickupSound`) (`self.CalculatedLocation`) (struct) 1.0 1.0 0.0 null null null null)))))
    (:`Finished`
      (`self.StartSinusoidalMovement`)
      (`self.StartRotation`))))

(event `self.ReceiveTick`
  (params (DeltaSeconds :type "Float (single-precision)"))
  (`self.K2_SetActorLocationAndRotation` (`self.CalculatedLocation`) (`self.CalculatedRotation`)))

(event `self.ReceiveDestroyed`
  (`GameplayStatics.PlaySoundAtLocation` (`self.ConsumeSound`) (`self.K2_GetActorLocation`) (struct) 1.0 1.0 0.0 null null null null))

(fn `CalculateDrop`
  (params (Drop :type "Float (double-precision)"))
  (returns (DropLocation :type "Vector Structure"))
  (bind (_initiallocation_x _initiallocation_y _initiallocation_z) (`KismetMathLibrary.BreakVector` (`self.InitialLocation`)))
  (return (`KismetMathLibrary.MakeVector` _initiallocation_x _initiallocation_y (+ _initiallocation_z (* Drop (`self.DropApex`))))))

(fn `UserConstructionScript`)